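; BP_Medium is a third-person shooter player character with Enhanced Input movement, camera, jump, crouch, sprint and a HUD.
; Aiming shortens the camera arm via timeline and switches fire from rapid shots to a costlier single shot on a longer cooldown.
; Shots are debug-drawn muzzle traces along camera forward, gated by DoOnce and Delay, with no damage applied.
; The railgun ultimate disables movement without restoring it, then capsule-traces after a delay.
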(event Custom|Ultimate
  (bind _rifle (Variables|Default|GetRifle))
  (bind _returnvalue (Transformation|GetSocketTransform _rifle "b_gun_muzzleflash" "RTS_World"))
  ;[1 1 1] Ultimate Railgun - TODO: Re-enable movement, maybe add timeline to slow down movement instead of just stopping?
  (Utilities|FlowControl|DoOnce false :!label _label
    (:Completed
      (Utilities|FlowControl|Sequence
        (:then_0
          (Pawn|Components|CharacterMovement|DisableMovement (Variables|Character|GetCharacterMovement))
          (Utilities|FlowControl|Delay 0.67)
          (Collision|CapsuleTraceByChannel (.location _returnvalue) (+ (.location _returnvalue) (* (Math|Vector|GetForwardVector (Transformation|GetWorldRotation (Variables|Default|GetCamera))) 4e+03)) 3e+01 0.0 "TraceTypeQuery1" false 0 "ForDuration"))
        (:then_1
          (Utilities|FlowControl|Delay 2.0)
          (goto _label Reset))))))

(event Custom|Regular%20Fire
  (bind _rifle (Variables|Default|GetRifle))
  (bind _returnvalue (Transformation|GetSocketTransform _rifle "b_gun_muzzleflash" "RTS_World"))
  ;[1 1 1] Code for rapid fire shooting
  (if (>= (Variables|Default|GetammoCount) 1)
    (Utilities|FlowControl|DoOnce false :!label _label
      (:Completed
        (Utilities|FlowControl|Sequence
          (:then_0
            (Collision|LineTraceByChannel (.location _returnvalue) (+ (.location _returnvalue) (* (Math|Vector|GetForwardVector (Transformation|GetWorldRotation (Variables|Default|GetCamera))) 4e+03)) "TraceTypeQuery1" false 0 "ForDuration")
            (Variables|Default|SetammoCount (- (Variables|Default|GetammoCount) 1)))
          (:then_1
            (Utilities|FlowControl|Delay 0.05)
            (goto _label Reset)))))))

(event Custom|Single%20Fire
  (bind _rifle (Variables|Default|GetRifle))
  (bind _returnvalue (Transformation|GetSocketTransform _rifle "b_gun_muzzleflash" "RTS_World"))
  ;[1 1 1] Code for single fire shooting - on a 5 second cooldown
  (if (>= (Variables|Default|GetammoCount) 5)
    (Utilities|FlowControl|DoOnce false :!label _label
      (:Completed
        (Utilities|FlowControl|Sequence
          (:then_0
            (Collision|LineTraceByChannel (.location _returnvalue) (+ (.location _returnvalue) (* (Math|Vector|GetForwardVector (Transformation|GetWorldRotation (Variables|Default|GetCamera))) 4e+03)) "TraceTypeQuery1" false 0 "ForDuration")
            (Variables|Default|SetammoCount (- (Variables|Default|GetammoCount) 5)))
          (:then_1
            (Utilities|FlowControl|Delay 5.0)
            (goto _label Reset)))))))

(event Input|EnhancedActionEvents|EnhancedInputActionINP_Jump
  (params (ActionValue :type Boolean) (ElapsedSeconds :type Float%20%28double-precision%29) (TriggeredSeconds :type Float%20%28double-precision%29) (InputAction :type Input%20Action%20Object%20Reference :default "/Game/AGraber/Input/Actions/INP_Jump.INP_Jump"))
  ;[1 1 1] Controls Player Jumping, set up in case jump hold wants to be set up
  (:Started
    (Character|Jump))
  (:Completed
    (Character|StopJumping)))

(event Input|EnhancedActionEvents|EnhancedInputActionINP_MovePlayer
  (params (ActionValue :type Vector%202D%20Structure) (ElapsedSeconds :type Float%20%28double-precision%29) (TriggeredSeconds :type Float%20%28double-precision%29) (InputAction :type Input%20Action%20Object%20Reference :default "/Game/AGraber/Input/Actions/INP_MovePlayer.INP_MovePlayer"))
  (bind _returnvalue (Pawn|GetControlRotation :!class /Script/Engine.Pawn))
  ;[1 1 1] Controls movement of player
  (:Triggered
    (Pawn|Input|AddMovementInput (Math|Vector|GetRightVector (Pawn|GetControlRotation :!class /Script/Engine.Pawn)) (.x ActionValue) false)
    (Pawn|Input|AddMovementInput (Math|Vector|GetForwardVector (Math|Rotator|MakeRotator (.roll _returnvalue) 0.0 (.yaw _returnvalue))) (.y ActionValue) false)))

(event Input|EnhancedActionEvents|EnhancedInputActionINP_Reload
  (params (ActionValue :type Boolean) (ElapsedSeconds :type Float%20%28double-precision%29) (TriggeredSeconds :type Float%20%28double-precision%29) (InputAction :type Input%20Action%20Object%20Reference :default "/Game/AGraber/Input/Actions/INP_Reload.INP_Reload"))
  ;[1 1 1] Base code for reloading
  (:Started
    (if (== (Variables|Default|GetammoCount) 30)
      (Variables|Default|SetammoCount 31)
      (else
        (Variables|Default|SetammoCount 30)))))

(event Input|EnhancedActionEvents|EnhancedInputActionINP_LookAround
  (params (ActionValue :type Vector%202D%20Structure) (ElapsedSeconds :type Float%20%28double-precision%29) (TriggeredSeconds :type Float%20%28double-precision%29) (InputAction :type Input%20Action%20Object%20Reference :default "/Game/AGraber/Input/Actions/INP_LookAround.INP_LookAround"))
  ;[1 1 1] Player Camera
  (:Triggered
    (Pawn|Input|AddControllerYawInput (* (.x ActionValue) (Math|Float|SelectFloat -1.0 1.0 (Variables|Default|GetInvertCamX))))
    (Pawn|Input|AddControllerPitchInput (* (.y ActionValue) (Math|Float|SelectFloat -1.0 1.0 (Variables|Default|GetInvertCamY))))))

(event Input|EnhancedActionEvents|EnhancedInputActionINP_Sprint
  (params (ActionValue :type Boolean) (ElapsedSeconds :type Float%20%28double-precision%29) (TriggeredSeconds :type Float%20%28double-precision%29) (InputAction :type Input%20Action%20Object%20Reference :default "/Game/AGraber/Input/Actions/INP_Sprint.INP_Sprint"))
  ;[1 1 1] Code for sprinting - if these values change make sure to update animation values too
  (:Triggered
    (if ActionValue
      (Variables|/Script/Engine.CharacterMovementComponent|SetMaxWalkSpeed (Variables|Character|GetCharacterMovement) 6e+02)
      (Variables|Default|SetisSprinting true)
      (else
        (Variables|/Script/Engine.CharacterMovementComponent|SetMaxWalkSpeed (Variables|Character|GetCharacterMovement) 3e+02)
        (Variables|Default|SetisSprinting false)))))

(event Input|EnhancedActionEvents|EnhancedInputActionINP_Crouch
  (params (ActionValue :type Boolean) (ElapsedSeconds :type Float%20%28double-precision%29) (TriggeredSeconds :type Float%20%28double-precision%29) (InputAction :type Input%20Action%20Object%20Reference :default "/Game/AGraber/Input/Actions/INP_Crouch.INP_Crouch"))
  ;[1 1 1] Crouching - TODO: Add code to slide
  (:Started
    (if (not (Variables|Default|GetisSprinting))
      (Character|Crouch)))
  (:Completed
    (Character|UnCrouch)))

(event Input|EnhancedActionEvents|EnhancedInputActionINP_ADS
  (params (ActionValue :type Boolean) (ElapsedSeconds :type Float%20%28double-precision%29) (TriggeredSeconds :type Float%20%28double-precision%29) (InputAction :type Input%20Action%20Object%20Reference :default "/Game/AGraber/Input/Actions/INP_ADS.INP_ADS"))
  (bind _charactermovement (Variables|Character|GetCharacterMovement))
  (bind _charactermovement_2 (Variables|Character|GetCharacterMovement))
  ;[1 1 1] Right Click Aiming - will always orient player to camera focus, even if something breaks
  (:Started
    (Variables|Default|SetisAiming true)
    (Variables|/Script/Engine.CharacterMovementComponent|SetbOrientRotationToMovement _charactermovement_2 false)
    (Variables|/Script/Engine.CharacterMovementComponent|SetbUseControllerDesiredRotation _charactermovement_2 true)
    (bind _camarmlength (Timeline|Aiming Play)
      (:Update
        (Variables|/Script/Engine.SpringArmComponent|SetTargetArmLength (Variables|Default|GetSelfieStick) (Math|Float|Lerp 55.0 2e+01 _camarmlength)))))
  (:Completed
    (Variables|Default|SetisAiming false)
    (Variables|/Script/Engine.CharacterMovementComponent|SetbOrientRotationToMovement _charactermovement true)
    (Variables|/Script/Engine.CharacterMovementComponent|SetbUseControllerDesiredRotation _charactermovement false)
    (Timeline|Aiming Reverse)))

(event Input|EnhancedActionEvents|EnhancedInputActionINP_Tactical
  (params (ActionValue :type Boolean) (ElapsedSeconds :type Float%20%28double-precision%29) (TriggeredSeconds :type Float%20%28double-precision%29) (InputAction :type Input%20Action%20Object%20Reference :default "/Game/AGraber/Input/Actions/INP_Tactical.INP_Tactical"))
  ;[1 1 1] Beginner code for Tactical ability
)

(event Input|EnhancedActionEvents|EnhancedInputActionINP_Fire
  (params (ActionValue :type Boolean) (ElapsedSeconds :type Float%20%28double-precision%29) (TriggeredSeconds :type Float%20%28double-precision%29) (InputAction :type Input%20Action%20Object%20Reference :default "/Game/AGraber/Input/Actions/INP_Fire.INP_Fire"))
  ;[1 1 1] Toggles between single fire (high powered shot) and rapid fire (low damage) if aiming down sights
  (:Triggered
    (if (Variables|Default|GetisAiming)
      (CallFunction|SingleFire)
      (else
        (CallFunction|RegularFire)))))

(event Input|EnhancedActionEvents|EnhancedInputActionINP_Ultimate
  (params (ActionValue :type Boolean) (ElapsedSeconds :type Float%20%28double-precision%29) (TriggeredSeconds :type Float%20%28double-precision%29) (InputAction :type Input%20Action%20Object%20Reference :default "/Game/AGraber/Input/Actions/INP_Ultimate.INP_Ultimate"))
  ;[1 1 1] Code for performing ultimate - TODO: Show cooldown of ability
  (:Started
    (CallFunction|Ultimate)))

(event EventBeginPlay
  (bind _returnvalue (Game|GetPlayerController 0))
  (bind _returnvalue_2 (PlayerController|LocalPlayerSubsystems|GetEnhancedInputLocalPlayerSubsystem _returnvalue))
  ;[1 1 1] Sets up Enhanced Input System
  (Utilities|IsValid _returnvalue_2
    (:Is%20Valid
      (Input|AddMappingContext _returnvalue_2 "/Game/AGraber/Input/Mappings/IMC_ThirdPerson.IMC_ThirdPerson" 0 "(bIgnoreAllPressedKeysUntilRelease=True,bForceImmediately=False)")
      (bind _returnvalue_3 (UserInterface|CreateWidget "/Game/AGraber/Widgets/WB_HUD.WB_HUD_C"))
      (UserInterface|Viewport|AddtoViewport _returnvalue_3 0)
      (Variables|Default|SetammoCount 30))))

(event Collision|EventActorBeginOverlap
  (params (OtherActor :type Actor%20Object%20Reference)))

(event EventTick
  (params (DeltaSeconds :type Float%20%28single-precision%29)))

(fn ConstructionScript)